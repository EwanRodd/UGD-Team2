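; Base gun Blueprint that fires BP_Projectile actors from its Arrow component.
; Fire is gated by CanFire and Reload, and RateOfFire re-enables CanFire through a fixed retriggerable delay.
; A zero bullet count sets Reload, but the GunType write-back subtracts zero from BulletCount and resets other fields to literals.
; A camera-channel line trace is left unconnected, and spawn locations are printed for debugging.
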(event `RateOfFire`
  (`KismetSystemLibrary.RetriggerableDelay` 0.2)
  (set `self.CanFire` true))

(event `self.ReceiveBeginPlay`
  (set `self.GunType` (struct)))

(event `Fire`
  (params (Gun :type "/Game/Equipable_Items/GunType_S Structure"))
  (bind (_guntype_gunname _guntype_bulletcountmax _guntype_bulletcount) (break `/Game/Equipable_Items/GunType_S` (`self.GunType`)))
  (if (`self.CanFire`)
    (if (not (`self.Reload`))
      (set `self.CanFire` false)
      (bind _returnvalue (`|SpawnActorFromClass` "/Game/BP_Projectile.BP_Projectile_C" (`SceneComponent.K2_GetComponentToWorld` (`self.Arrow`)) "AlwaysSpawn" "MultiplyWithRoot" null null))
      (bind _returnvalue_location (`KismetMathLibrary.BreakTransform` (`self.GetTransform` _returnvalue)))
      (`KismetSystemLibrary.PrintString` (`KismetStringLibrary.Conv_VectorToString` _returnvalue_location))
      (`self.RateOfFire`)
      (if (== _guntype_bulletcount 0)
        (set `self.Reload` true)
        (else
          (set `self.Reload` false)))
      (set `self.GunType` (make `/Game/Equipable_Items/GunType_S` "" 0 (`KismetMathLibrary.FTrunc` (- _guntype_bulletcount 0.0)) 0.0 0 0.0 null null null)))))

(fn `NewFunction`)

(fn `UserConstructionScript`)