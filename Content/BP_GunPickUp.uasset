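; BP_GunPickUp is a world gun pickup that the first-person character can add to their inventory.
; BeginPlay fills its gun info struct with hardcoded defaults.
; Each Tick polls the sphere with a component overlap query rather than overlap events, looking for the player character.
; If that player's interact flag is set, it passes the gun type and info to their inventory, prints the pickup class name and destroys itself.
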(event `self.ReceiveBeginPlay`
  (set `self.GunTypeInfo` (make `/Game/Equipable_Items/GunType_S` "" 10 10 1.0 5 5.0 "/Game/Equipable_Items/Models/Blaster_1/SKM_blaster-a.SKM_blaster-a" "/Game/BP_GunBase.BP_GunBase_C" "BP_GunPickUp_C")))

(event `self.ReceiveTick`
  (params (DeltaSeconds :type "Float (single-precision)"))
  (bind _sphere (`self.Sphere`))
  ; Overlaping
  (bind (_outactors _returnvalue) (`KismetSystemLibrary.ComponentOverlapActors` _sphere (`SceneComponent.K2_GetComponentToWorld` _sphere) (`self.Object Types`)))
  (for _array_element _outactors
    (if _returnvalue
      (bind _asbp_first_person_character (cast `/Game/FirstPerson/Blueprints/BP_FirstPersonCharacter` _array_element))
      (`self.OverLap` _asbp_first_person_character)
      (break))))

(event `OverLap`
  (params (PlayerBody :type "/Game/FirstPerson/Blueprints/BP_FirstPersonCharacter Object Reference"))
  (bind (_guntypeinfo_gunname _guntypeinfo_bulletcountmax _guntypeinfo_bulletcount _guntypeinfo_rateoffire _guntypeinfo_magizines _guntypeinfo_reload _guntypeinfo_skelatal _guntypeinfo_gunbase _guntypeinfo_gunpickup) (break `/Game/Equipable_Items/GunType_S` (`self.GunTypeInfo`)))
  ; Equip button pressed
  (if (`/Game/FirstPerson/Blueprints/BP_FirstPersonCharacter.IsInteract` PlayerBody)
    (`/Game/Equipable_Items/BP_Inventory.PickUpGun` (`/Game/FirstPerson/Blueprints/BP_FirstPersonCharacter.BP_Inventory` PlayerBody) (`self.GunType`) (`self.GunTypeInfo`))
    (`KismetSystemLibrary.PrintString` (`KismetSystemLibrary.GetClassDisplayName` _guntypeinfo_gunpickup))
    (`self.K2_DestroyActor`)))

(fn `UserConstructionScript`)