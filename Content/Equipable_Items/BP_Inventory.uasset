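; Inventory on the first-person character that holds a two-gun loadout and swaps between the held and backup weapon.
; Initalise caches the owning character and HUD, then equips the starting gun through the weapon component.
; Switch exchanges guns using a boolean slot index, gated by a DoOnce that Completed resets.
; UpdateUI pushes both guns' images and ammo to the HUD, while Tick refreshes the held gun's bullet count.
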(event `Initalise`
  (bind (_startinggun_gunname _startinggun_bulletcountmax _startinggun_bulletcount _startinggun_rateoffire _startinggun_magizines _startinggun_reload _startinggun_skelatal _startinggun_gunbase _startinggun_gunpickup _startinggun_ispistol _startinggun_isriffle _startinggun_image) (break `/Game/Equipable_Items/GunType_S` (`self.StartingGun`)))
  (bind _startinggun (`self.StartingGun`))
  ; Casting
  (bind _asbp_first_person_character (cast `/Game/FirstPerson/Blueprints/BP_FirstPersonCharacter` (`self.GetOwner`))
    (:`then`
      (bind _output_get (set `self.As BP First Person Character` _asbp_first_person_character))
      (set `self.GunInHand` _startinggun)
      (`/Game/Equipable_Items/BP_WeaponComponent.ChangedGun` (`/Game/FirstPerson/Blueprints/BP_FirstPersonCharacter.BP_WeaponComponent` _output_get) _startinggun)
      (bind _output_get_2 (set `self.Hud` (`/Game/FirstPerson/Blueprints/BP_FirstPersonCharacter.Hud` _output_get)))
      (`/Game/Equipable_Items/HUD_UIW.SetCurrentGun` _output_get_2 _startinggun_image)
      (set `self.Guns` (`|MakeArray` (`self.GunInHand`) (`self.BackUpGun`)))
      (set `self.GunIndex` false)
      (`self.UpdateUI`))
    (:`CastFailed`
      (`KismetSystemLibrary.PrintString` "Failed"))))

(event `self.ReceiveTick`
  (params (DeltaSeconds :type "Float (single-precision)"))
  (bind (_guninhand_gunname _guninhand_bulletcountmax _guninhand_bulletcount) (break `/Game/Equipable_Items/GunType_S` (`self.GunInHand`)))
  (`/Game/Equipable_Items/HUD_UIW.SetCurrentBulletCount ` (`self.Hud`) _guninhand_bulletcount))

(event `Switch`
  (bind _guns (`self.Guns`))
  (bind _guninhand (`self.GunInHand`))
  (bind _tempgun (`self.TempGun`))
  (bind _bp_weaponcomponent (`/Game/FirstPerson/Blueprints/BP_FirstPersonCharacter.BP_WeaponComponent` (`self.As BP First Person Character`)))
  (`/Engine/EditorBlueprintResources/StandardMacros.DoOnce` false :!label _label
    (:`Completed`
      (set `self.TempGun` (`self.GunInHand`))
      (if (`self.GunIndex`)
        (set `self.GunInHand` (`|GetArrayItem` (`self.Guns`)))
        (`KismetArrayLibrary.Array_Set` _guns 1 _tempgun)
        (`/Game/Equipable_Items/BP_WeaponComponent.ChangedGun` _bp_weaponcomponent _guninhand)
        (`self.UpdateUI`)
        (set `self.GunIndex` false)
        (else
          (set `self.GunInHand` (`|GetArrayItem` (`self.Guns`) 1))
          (`KismetArrayLibrary.Array_Set` _guns 0 _tempgun)
          (`/Game/Equipable_Items/BP_WeaponComponent.ChangedGun` _bp_weaponcomponent _guninhand)
          (`self.UpdateUI`)
          (set `self.GunIndex` true))))))

(event `Completed`
  (goto _label :!via `Reset`))

(fn `UpdateUI`
  (bind _hud (`self.Hud`))
  (bind (_guninhand_gunname _guninhand_bulletcountmax _guninhand_bulletcount _guninhand_rateoffire _guninhand_magizines _guninhand_reload _guninhand_skelatal _guninhand_gunbase _guninhand_gunpickup _guninhand_ispistol _guninhand_isriffle _guninhand_image) (break `/Game/Equipable_Items/GunType_S` (`self.GunInHand`)))
  (bind (_output_gunname _output_bulletcountmax _output_bulletcount _output_rateoffire _output_magizines _output_reload _output_skelatal _output_gunbase _output_gunpickup _output_ispistol _output_isriffle _output_image) (break `/Game/Equipable_Items/GunType_S` (`|GetArrayItem` (`self.Guns`) (`self.index`))))
  (`/Game/Equipable_Items/HUD_UIW.SetCurrentGun` _hud _guninhand_image)
  (`/Game/Equipable_Items/HUD_UIW.SetCurrentMagCount` _hud _guninhand_magizines)
  (if (`self.GunIndex`)
    (set `self.index` 1)
    (`/Game/Equipable_Items/HUD_UIW.SetBackUpBulletCount` _hud _output_bulletcount)
    (`/Game/Equipable_Items/HUD_UIW.SetBackUpGun` _hud _output_image)
    (`/Game/Equipable_Items/HUD_UIW.SetBackUpMagCount` _hud _output_magizines)
    (else
      (`KismetSystemLibrary.PrintString` _output_gunname)
      (set `self.index` 0)
      (`/Game/Equipable_Items/HUD_UIW.SetBackUpBulletCount` _hud _output_bulletcount)
      (`/Game/Equipable_Items/HUD_UIW.SetBackUpGun` _hud _output_image)
      (`/Game/Equipable_Items/HUD_UIW.SetBackUpMagCount` _hud _output_magizines))))