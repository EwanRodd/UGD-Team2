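; Base gun actor that fires hitscan shots at zombies and tracks its own ammo.
; Fire is gated by ready, reload and empty flags, with delays timing fire rate and magazine reloads, and copies the updated GunType struct to the owner's Inventory.
; A camera line trace with slight random offset damages Zombie-tagged actors or spawns a decal on other hit actors.
; Sound and particle effects play only when the trace hits an actor.
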(event `Initalise`
  (params (inventory :type "/Game/Equipable_Items/BP_Inventory Object Reference"))
  ; Casting
  (set `self.Inventory` inventory)
  (cast `/Game/FirstPerson/Blueprints/BP_FirstPersonCharacter` (`self.GetOwner`))
  (set `self.As BP First Person Character` (`self.As BP First Person Character`)))

(event `ReloadTimer`
  (bind (_guntype_gunname _guntype_bulletcountmax _guntype_bulletcount _guntype_rateoffire _guntype_magizines _guntype_reload _guntype_skelatal _guntype_gunbase _guntype_gunpickup _guntype_ispistol _guntype_isriffle _guntype_image) (break `/Game/Equipable_Items/GunType_S` (`self.GunType`)))
  ; Reload
  (`KismetSystemLibrary.Delay` _guntype_reload)
  (set `self.Reload` false)
  (bind _output_get (set `self.GunType` (make `/Game/Equipable_Items/GunType_S` _guntype_gunname _guntype_bulletcountmax _guntype_bulletcountmax _guntype_rateoffire (- _guntype_magizines 1) _guntype_reload _guntype_skelatal _guntype_gunbase _guntype_gunpickup _guntype_ispistol _guntype_isriffle _guntype_image)))
  (set `/Game/Equipable_Items/BP_Inventory.GunInHand` _output_get (`self.Inventory`))
  (set `self.CanFire` true))

(event `RateOfFire`
  (bind (_guntype_gunname _guntype_bulletcountmax _guntype_bulletcount _guntype_rateoffire) (break `/Game/Equipable_Items/GunType_S` (`self.GunType`)))
  ; RateOfFire
  (if (not (`self.Reload`))
    (`KismetSystemLibrary.Delay` _guntype_rateoffire)
    (set `self.CanFire` true)))

(event `NewGun`
  (params (NewGun :type "/Game/Equipable_Items/GunType_S Structure"))
  (set `self.GunType` NewGun))

(event `Fire`
  (bind (_guntype_gunname _guntype_bulletcountmax _guntype_bulletcount _guntype_rateoffire _guntype_magizines _guntype_reload _guntype_skelatal _guntype_gunbase _guntype_gunpickup _guntype_ispistol _guntype_isriffle _guntype_image) (break `/Game/Equipable_Items/GunType_S` (`self.GunType`)))
  (bind (_guntype_gunname_2 _guntype_bulletcountmax_2 _guntype_bulletcount_2 _guntype_rateoffire_2 _guntype_magizines_2) (break `/Game/Equipable_Items/GunType_S` (`self.GunType`)))
  (if (`self.CanFire`)
    (if (`self.Reload`)
      _
      (elif (not (`self.Empty`))
        (set `self.CanFire` false)
        (`self.LineTrace`)
        (`self.RateOfFire`)
        (if (== _guntype_bulletcount_2 0)
          (set `self.Reload` true)
          (set `self.CanFire` false)
          (`self.ReloadTimer`)
          (else
            (set `self.Reload` false)
            (set `self.Empty` (== _guntype_magizines_2 0))))
        (if (not (`self.Reload`))
          (bind _output_get (set `self.GunType` (make `/Game/Equipable_Items/GunType_S` _guntype_gunname _guntype_bulletcountmax (`KismetMathLibrary.Conv_Int64ToInt` (- _guntype_bulletcount_2 (`self.BulletMinus`))) _guntype_rateoffire _guntype_magizines _guntype_reload _guntype_skelatal _guntype_gunbase _guntype_gunpickup _guntype_ispistol _guntype_isriffle _guntype_image)))
          (set `/Game/Equipable_Items/BP_Inventory.GunInHand` _output_get (`self.Inventory`)))))))

(fn `LineTrace`
  (locals (NewLocalVar :type "/Game/Zombie/Zombie Object Reference"))
  (bind _returnvalue (`GameplayStatics.GetPlayerCameraManager` 0))
  (bind _returnvalue_2 (`PlayerCameraManager.GetCameraRotation` _returnvalue))
  (bind _returnvalue_location (`KismetMathLibrary.BreakTransform` (`SceneComponent.K2_GetComponentToWorld` (`Actor.RootComponent` _returnvalue))))
  (bind _outhit (`KismetSystemLibrary.LineTraceSingle` :`Start` _returnvalue_location :`End` (+ _returnvalue_location (* (`self.GetActorForwardVector` _returnvalue) 10000000000000.0) (`KismetMathLibrary.Normal` (+ (`KismetMathLibrary.GetForwardVector` _returnvalue_2) (* (`KismetMathLibrary.GetRightVector` _returnvalue_2) (`KismetMathLibrary.RandomFloatInRange` 0.5 1.0)) (* (`KismetMathLibrary.GetUpVector` _returnvalue_2) (`KismetMathLibrary.RandomFloatInRange` 10.0 1.0))))) :`TraceChannel` "TraceTypeQuery1" :`DrawTime` 1.0))
  (bind (_bblockinghit _binitialoverlap _time _distance _location _impactpoint _normal _impactnormal _physmat _hitactor) (`GameplayStatics.BreakHitResult` _outhit))
  (`/Engine/EditorBlueprintResources/StandardMacros.IsValid` _hitactor
    (:`Is Valid`
      (if (`self.ActorHasTag` _hitactor "Zombie")
        (bind _aszombie (cast `/Game/Zombie/Zombie` _hitactor)
          (:`then`
            (`KismetSystemLibrary.PrintString` "done")
            (`/Game/Zombie/Zombie.Hit` _aszombie 50.0)
            (`self.SoundEffect` :!label _label)
            (`self.ParticleAffect`)
            (return))
          (:`CastFailed`
            (`KismetSystemLibrary.PrintString` "failed")))
        (else
          (`|SpawnActorFromClass` "/Game/Equipable_Items/Models/Decal.Decal_C" (`KismetMathLibrary.MakeTransform` _location (`KismetMathLibrary.MakeRotFromY` _impactnormal)) "Undefined" "MultiplyWithRoot" null null)
          (goto _label))))))

(fn `ParticleAffect`
  (bind (_returnvalue_location _returnvalue_rotation _returnvalue_scale) (`KismetMathLibrary.BreakTransform` (`SceneComponent.K2_GetComponentToWorld` (`self.Arrow`))))
  (`NiagaraFunctionLibrary.SpawnSystemAtLocation` null _returnvalue_location _returnvalue_rotation _returnvalue_scale)
  (return))

(fn `SoundEffect`
  (bind (_returnvalue_location _returnvalue_rotation) (`KismetMathLibrary.BreakTransform` (`SceneComponent.K2_GetComponentToWorld` (`self.SkeletalMesh`))))
  (`GameplayStatics.PlaySoundAtLocation` "/Game/SoundFX/universfield-gunshot-352466.universfield-gunshot-352466" _returnvalue_location _returnvalue_rotation (`KismetMathLibrary.RandomFloatInRange` 1.0 5.0) 1.0 0.0 null null null null)
  (return))

(fn `UserConstructionScript`)