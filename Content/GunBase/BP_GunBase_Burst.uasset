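; Burst-fire gun Blueprint that fires hitscan shots from the player camera and damages zombies.
; LineTrace and a delayed custom event call each other until Index reaches Burst, then reset it and set BulletMinus.
; Tagged zombies receive Hit, other actors get a decal, and both trigger sound and particle effects.
; The random spread is a normalized offset added to a very distant endpoint, so it barely affects aim.
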(event `self.ReceiveBeginPlay`
  (set `self.Burst` 5.0)
  (set `self.Index` 0.0))

(event `Delay`
  (`KismetSystemLibrary.Delay` 0.2)
  (set `self.Index` (+ (`self.Index`) 1.0))
  (`self.LineTrace`))

(fn `LineTrace`
  (bind _returnvalue (`GameplayStatics.GetPlayerCameraManager` 0))
  (bind _returnvalue_2 (`PlayerCameraManager.GetCameraRotation` _returnvalue))
  (bind _returnvalue_location (`KismetMathLibrary.BreakTransform` (`SceneComponent.K2_GetComponentToWorld` (`Actor.RootComponent` _returnvalue))))
  (if (!= (`self.Index`) (`self.Burst`))
    (bind _outhit (`KismetSystemLibrary.LineTraceSingle` :`Start` _returnvalue_location :`End` (+ _returnvalue_location (* (`self.GetActorForwardVector` _returnvalue) 10000000000000.0) (`KismetMathLibrary.Normal` (+ (`KismetMathLibrary.GetForwardVector` _returnvalue_2) (* (`KismetMathLibrary.GetRightVector` _returnvalue_2) (`KismetMathLibrary.RandomFloatInRange` 0.5 1.0)) (* (`KismetMathLibrary.GetUpVector` _returnvalue_2) (`KismetMathLibrary.RandomFloatInRange` 10.0 1.0))))) :`TraceChannel` "TraceTypeQuery1" :`DrawTime` 1.0))
    (bind (_bblockinghit _binitialoverlap _time _distance _location _impactpoint _normal _impactnormal _physmat _hitactor) (`GameplayStatics.BreakHitResult` _outhit))
    (`/Engine/EditorBlueprintResources/StandardMacros.IsValid` _hitactor
      (:`Is Valid`
        (if (`self.ActorHasTag` _hitactor "Zombie")
          (bind _aszombie (cast `/Game/Zombie/Zombie` _hitactor)
            (:`then`
              (`KismetSystemLibrary.PrintString` "done")
              (`/Game/Zombie/Zombie.Hit` _aszombie 50.0)
              (`self.SoundEffect` :!label _label)
              (`self.ParticleAffect`)
              (`self.Delay` :!label _label_2))
            (:`CastFailed`
              (`KismetSystemLibrary.PrintString` "failed")))
          (else
            (`|SpawnActorFromClass` "/Game/Equipable_Items/Models/Decal.Decal_C" (`KismetMathLibrary.MakeTransform` _location (`KismetMathLibrary.MakeRotFromY` _impactnormal)) "Undefined" "MultiplyWithRoot" null null)
            (goto _label))))
      (:`Is Not Valid`
        (goto _label_2)))
    (else
      (set `self.Index` 0.0)
      (set `self.BulletMinus` 5)
      (return))))

(fn `UserConstructionScript`
  (`parent.UserConstructionScript`))