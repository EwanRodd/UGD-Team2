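; Shotgun variant of the gun base that overrides the shot trace to fire a burst of spread pellets.
; Each pellet line-traces from the camera along its forward vector, with a random, positive-only per-axis offset up to Spread added to the end point.
; Hits on Zombie-tagged actors apply damage through Hit, while other valid hits spawn a decal.
; Sound and particle effects play once after all traces.
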(fn `LineTrace`
  (bind _transformcomponent (`PlayerCameraManager.TransformComponent` (`GameplayStatics.GetPlayerCameraManager` 0)))
  (bind _returnvalue (`SceneComponent.K2_GetComponentLocation` _transformcomponent))
  (for _ (range 11)
    (bind _outhit (`KismetSystemLibrary.LineTraceSingle` :`Start` _returnvalue :`End` (+ _returnvalue (* (`SceneComponent.GetForwardVector` _transformcomponent) 1000.0) (`KismetMathLibrary.MakeVector` (`KismetMathLibrary.RandomFloatInRange` 0.0 (`self.Spread`)) (`KismetMathLibrary.RandomFloatInRange` 0.0 (`self.Spread`)) (`KismetMathLibrary.RandomFloatInRange` 0.0 (`self.Spread`)))) :`TraceChannel` "TraceTypeQuery1" :`DrawTime` 1.0))
    (bind (_bblockinghit _binitialoverlap _time _distance _location _impactpoint _normal _impactnormal _physmat _hitactor) (`GameplayStatics.BreakHitResult` _outhit))
    (`/Engine/EditorBlueprintResources/StandardMacros.IsValid` _hitactor
      (:`Is Valid`
        (if (`self.ActorHasTag` _hitactor "Zombie")
          (bind _aszombie (cast `/Game/Zombie/Zombie` _hitactor)
            (:`then`
              (`KismetSystemLibrary.PrintString` "done")
              (`/Game/Zombie/Zombie.Hit` _aszombie 50.0))
            (:`CastFailed`
              (`KismetSystemLibrary.PrintString` "failed")))
          (else
            (`|SpawnActorFromClass` "/Game/Equipable_Items/Models/Decal.Decal_C" (`KismetMathLibrary.MakeTransform` _location (`KismetMathLibrary.MakeRotFromY` _impactnormal)) "Undefined" "MultiplyWithRoot" null null))))))
  (`self.SoundEffect`)
  (`self.ParticleAffect`)
  (return))

(fn `UserConstructionScript`
  (`parent.UserConstructionScript`))