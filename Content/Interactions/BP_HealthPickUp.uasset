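; Health pickup actor that spins around its yaw axis on Tick and is meant to heal the first-person character.
; A Box overlap matching the stored character reference passes a DoOnce, then adds Health without clamping if it is below the threshold.
; DestroyActor then targets the character rather than the pickup.
; The cast that sets the character reference is disconnected, so this graph never assigns it.
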(event `self.Box.OnComponentBeginOverlap`
  (params (OverlappedComponent :type "PrimitiveComponent Object Reference") (OtherActor :type "Actor Object Reference") (OtherComp :type "PrimitiveComponent Object Reference") (OtherBodyIndex :type Integer) (bFromSweep :type Boolean) (SweepResult :type "HitResult Structure (by ref)"))
  (bind _as_bp_first_person_character (`self.As BP First Person Character`))
  (if (== OtherActor (`self.As BP First Person Character`))
    (`/Engine/EditorBlueprintResources/StandardMacros.DoOnce` false
      (:`Completed`
        (if (< (`/Game/FirstPerson/Blueprints/BP_FirstPersonCharacter.Health` (`self.As BP First Person Character`)) 100.0)
          (set `/Game/FirstPerson/Blueprints/BP_FirstPersonCharacter.Health` (+ (`/Game/FirstPerson/Blueprints/BP_FirstPersonCharacter.Health` _as_bp_first_person_character) 20.0) _as_bp_first_person_character)
          (`self.K2_DestroyActor` (`self.As BP First Person Character`)))))))

(event `self.ReceiveTick`
  (params (DeltaSeconds :type "Float (single-precision)"))
  (`self.K2_AddActorLocalRotation` (`KismetMathLibrary.MakeRotator` 0.0 0.0 (* DeltaSeconds 50.0))))

(fn `UserConstructionScript`)