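; BP_SpinTrap is a hazard actor that spins around its pitch axis and ragdolls the first-person player on contact.
; Nothing here calls the SpinTrap event; once triggered, it re-arms a very short looping timer on itself and adds delta-time-scaled local rotation on each call, instead of using Tick.
; Two box components independently detect overlaps, cast to BP_FirstPersonCharacter and call its Ragdoll function.
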(event `SpinTrap`
  (`KismetSystemLibrary.K2_SetTimerDelegate` (delegate `SpinTrap`) 0.001 true)
  (`self.K2_AddActorLocalRotation` (`KismetMathLibrary.MakeRotator` 0.0 (* (`GameplayStatics.GetWorldDeltaSeconds`) 500.0))))

(event `self.Box.OnComponentBeginOverlap`
  (params (OverlappedComponent :type "PrimitiveComponent Object Reference") (OtherActor :type "Actor Object Reference") (OtherComp :type "PrimitiveComponent Object Reference") (OtherBodyIndex :type Integer) (bFromSweep :type Boolean) (SweepResult :type "HitResult Structure (by ref)"))
  (bind _asbp_first_person_character (cast `/Game/FirstPerson/Blueprints/BP_FirstPersonCharacter` OtherActor))
  (`/Game/FirstPerson/Blueprints/BP_FirstPersonCharacter.Ragdoll` _asbp_first_person_character))

(event `self.Box1.OnComponentBeginOverlap`
  (params (OverlappedComponent :type "PrimitiveComponent Object Reference") (OtherActor :type "Actor Object Reference") (OtherComp :type "PrimitiveComponent Object Reference") (OtherBodyIndex :type Integer) (bFromSweep :type Boolean) (SweepResult :type "HitResult Structure (by ref)"))
  (bind _asbp_first_person_character (cast `/Game/FirstPerson/Blueprints/BP_FirstPersonCharacter` OtherActor))
  (`/Game/FirstPerson/Blueprints/BP_FirstPersonCharacter.Ragdoll` _asbp_first_person_character))

(fn `UserConstructionScript`)